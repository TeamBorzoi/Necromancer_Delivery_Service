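; BP_StreetLight is a street lamp actor that switches on and off with the time of day.
; On BeginPlay it caches the first BP_Sky actor in the level.
; Every Tick it reads the sky's TimeOfDay, treating 17:00 through 08:00 as night, although its graph comment says 18:00.
; It then toggles the spot light's visibility and swaps the mesh's lamp material between emissive and off.
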(event `self.ReceiveBeginPlay`
  (`self.Create Sky Reference`))

(event `self.ReceiveTick`
  (params (DeltaSeconds :type "Float (single-precision)"))
  (`self.update lights`))

(event `Create Sky Reference`
  ;[0 0 0] Creating References
  (bind _outactors (`GameplayStatics.GetAllActorsOfClass` "/Game/PizzaBoySystem/Blueprints/BP_Sky.BP_Sky_C"))
  (set `self.Sky` (`|GetArrayItem` _outactors)))

(event `update lights`
  (bind _spotlight (`self.SpotLight`))
  (bind _staticmesh (`self.StaticMesh`))
  (bind _time_of_day (`/Game/PizzaBoySystem/Blueprints/BP_Sky.Time of Day` (`self.Sky`)))
  ;[0 0 0] Update Vehicle Lights Between 18:00 and 08:00
  (if (or (>= _time_of_day 17.0) (<= _time_of_day 8.0))
    (`SceneComponent.SetVisibility` _spotlight true false)
    (`PrimitiveComponent.SetMaterial` _staticmesh 1 "/Game/PizzaBoySystem/Materials/M_Emissive.M_Emissive")
    (else
      (`SceneComponent.SetVisibility` _spotlight false false)
      (`PrimitiveComponent.SetMaterial` _staticmesh 1 "/Game/PizzaBoySystem/Materials/M_LampOff.M_LampOff"))))

(fn `UserConstructionScript`)