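; BP_EndMissionTrigger is the marker actor that ends an active pizza delivery mission once all deliveries are done.
; When the vehicle overlaps its sphere, it checks the game mode's mission flag and AllDelivered, then calls EndMission on the game mode.
; It then clears CanEnter on the delivery vehicle and disables itself through EnableMarker, which toggles both mesh visibility and actor collision.
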(event `Enable Marker`
  (params (Enabled :type Boolean))
  (bind _staticmesh (`self.StaticMesh`))
  (if Enabled
    (`SceneComponent.SetHiddenInGame` _staticmesh false false)
    (`self.SetActorEnableCollision` true)
    (else
      (`SceneComponent.SetHiddenInGame` _staticmesh true false)
      (`self.SetActorEnableCollision` false))))

(event `self.Sphere.OnComponentBeginOverlap`
  (params (OverlappedComponent :type "PrimitiveComponent Object Reference") (OtherActor :type "Actor Object Reference") (OtherComp :type "PrimitiveComponent Object Reference") (OtherBodyIndex :type Integer) (bFromSweep :type Boolean) (SweepResult :type "HitResult Structure (by ref)"))
  (bind _asbp_third_person_game_mode (`/Game/PizzaBoySystem/Blueprints/FunctionLibrary.Get Game Mode`))
  (bind _get_vehicle (`self.Get Vehicle`))
  (if (and (== OtherActor _get_vehicle) (`/Game/PizzaBoySystem/Blueprints/BP_GameMode.Pizza Mission Active?` _asbp_third_person_game_mode))
    (`/Game/PizzaBoySystem/Blueprints/ActorMacroLibrary.All Delivered`
      (:`true`
        (`/Game/PizzaBoySystem/Blueprints/BP_GameMode.End Mission` _asbp_third_person_game_mode true)
        (bind _asbp_delivery_vehicle (cast `/Game/PizzaBoySystem/Blueprints/BP_DeliveryVehicle` _get_vehicle))
        (set `/Game/PizzaBoySystem/Blueprints/BP_DeliveryVehicle.Can Enter?` false _asbp_delivery_vehicle)
        (`self.Enable Marker` false)))))

(fn `UserConstructionScript`)