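; Mission start marker for the Pizza Boy delivery job, with a toggle for its mesh visibility and collision.
; Player overlap with no pizza mission active checks BP_Sky's time of day, currently a full-day window, with a HUD closed notice otherwise.
; A delayed sequence fades a mission screen, teleports the player beside the marker, starts the timed GameMode mission, and enables the delivery vehicle's arrow and entry with a HUD prompt.
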(event `self.ReceiveBeginPlay`
  (bind _returnvalue (`GameplayStatics.GetActorOfClass` "/Game/PizzaBoySystem/Blueprints/BP_Sky.BP_Sky_C"))
  (set `self.BP_Sky` _returnvalue))

(event `Enable Marker`
  (params (Enabled :type Boolean))
  (bind _sm_marker (`self.SM_Marker`))
  (if Enabled
    (`SceneComponent.SetHiddenInGame` _sm_marker false false)
    (`self.SetActorEnableCollision` true)
    (else
      (`SceneComponent.SetHiddenInGame` _sm_marker true false)
      (`self.SetActorEnableCollision` false))))

(event `self.Sphere.OnComponentBeginOverlap`
  (params (OverlappedComponent :type "PrimitiveComponent Object Reference") (OtherActor :type "Actor Object Reference") (OtherComp :type "PrimitiveComponent Object Reference") (OtherBodyIndex :type Integer) (bFromSweep :type Boolean) (SweepResult :type "HitResult Structure (by ref)"))
  (bind _returnvalue (`/Game/PizzaBoySystem/Blueprints/FunctionLibrary.Get HUD`))
  (bind (_returnvalue_roll _returnvalue_pitch) (`KismetMathLibrary.BreakRotator` (`self.K2_GetActorRotation`)))
  (bind _get_vehicle (`self.Get Vehicle`))
  (if (and (== OtherActor (`GameplayStatics.GetPlayerCharacter` 0)) (not (`/Game/PizzaBoySystem/Blueprints/BP_GameMode.Pizza Mission Active?` (`/Game/PizzaBoySystem/Blueprints/FunctionLibrary.Get Game Mode`))))
    (if (`KismetMathLibrary.InRange_FloatFloat` (`/Game/PizzaBoySystem/Blueprints/BP_Sky.Time of Day` (`self.BP_Sky`)) 0.0 24.0)
      (bind _returnvalue_2 (`|CreateWidget` "/Game/PizzaBoySystem/Widgets/W_MissionScreen.W_MissionScreen_C" null "Pizza Boy"))
      (`UserWidget.AddToViewport` _returnvalue_2 0)
      (`/Game/PizzaBoySystem/Widgets/W_MissionScreen.Fade In` _returnvalue_2)
      (`KismetSystemLibrary.Delay` 1.0)
      (`self.K2_SetActorTransform` (`GameplayStatics.GetPlayerCharacter` 0) (`KismetMathLibrary.MakeTransform` (- (`self.K2_GetActorLocation`) (100.0 0.0 0.0)) (`KismetMathLibrary.MakeRotator` _returnvalue_roll _returnvalue_pitch -180.0)) false true)
      (`KismetSystemLibrary.Delay` 3.0)
      (`/Game/PizzaBoySystem/Widgets/W_MissionScreen.Fade Out` _returnvalue_2)
      (`/Game/PizzaBoySystem/Blueprints/BP_GameMode.Start Mission` (`/Game/PizzaBoySystem/Blueprints/FunctionLibrary.Get Game Mode`) (`/Game/PizzaBoySystem/Blueprints/BP_DeliveryVehicle.Delivery Points` _get_vehicle) (`self.Minutes`) (`self.Seconds`))
      (`/Game/PizzaBoySystem/Blueprints/BP_DeliveryVehicle.Spawn Arrow` _get_vehicle true)
      (`KismetSystemLibrary.Delay` 1.0)
      (`Widget.RemoveFromParent` _returnvalue_2)
      (set `/Game/PizzaBoySystem/Blueprints/BP_DeliveryVehicle.Can Enter?` true _get_vehicle)
      (`/Game/PizzaBoySystem/Blueprints/BP_HUD.Create Message 2` _returnvalue "Enter in the" "Delivery Vehicle" 0 30)
      (else
        (`/Game/PizzaBoySystem/Blueprints/BP_HUD.Closed` _returnvalue)))))

(fn `UserConstructionScript`)