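; Blueprint function library for the PizzaBoy delivery system that provides shortcuts to its core objects.
; Game instance, game mode and delivery vehicle getters cast to their project Blueprint classes, with the vehicle taken from player pawn 0.
; The HUD getter finds the first BP_HUD actor in the world.
; The delivery points getter returns every BP_DeliveryPoint actor in the level.
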(fn `Get Delivery Points`
  (returns (OutActors :type "Array of /Game/PizzaBoySystem/Blueprints/BP_DeliveryPoint Object Reference"))
  (bind _outactors (`GameplayStatics.GetAllActorsOfClass` null "/Game/PizzaBoySystem/Blueprints/BP_DeliveryPoint.BP_DeliveryPoint_C"))
  (return _outactors))

(fn `Get Delivery Vehicle`
  (returns (`AsSports Car Pawn` :type "/Game/PizzaBoySystem/Blueprints/BP_DeliveryVehicle Object Reference"))
  (bind _asbp_delivery_vehicle (cast `/Game/PizzaBoySystem/Blueprints/BP_DeliveryVehicle` (`GameplayStatics.GetPlayerPawn` null)))
  (return _asbp_delivery_vehicle))

(fn `Get Game Instance`
  (returns (`AsBP Game Instance` :type "/Game/PizzaBoySystem/Blueprints/BP_GameInstance Object Reference"))
  (bind _asbp_game_instance (cast `/Game/PizzaBoySystem/Blueprints/BP_GameInstance` (`GameplayStatics.GetGameInstance` null)))
  (return _asbp_game_instance))

(fn `Get Game Mode`
  (returns (`AsBP Third Person Game Mode` :type "/Game/PizzaBoySystem/Blueprints/BP_GameMode Object Reference"))
  (bind _asbp_game_mode (cast `/Game/PizzaBoySystem/Blueprints/BP_GameMode` (`GameplayStatics.GetGameMode` null)))
  (return _asbp_game_mode))

(fn `Get HUD`
  (returns (ReturnValue :type "/Game/PizzaBoySystem/Blueprints/BP_HUD Object Reference"))
  (bind _returnvalue (`GameplayStatics.GetActorOfClass` null "/Game/PizzaBoySystem/Blueprints/BP_HUD.BP_HUD_C"))
  (return _returnvalue))