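; Pizza delivery drop-off point that stays without collision until enabled and can be completed only once.
; When the delivery vehicle overlaps its sphere, it shows an interaction widget and opens a Gate for the E key.
; Delivering adds random earnings and a pizza count to the GameMode, then disables the point.
; Once all are delivered, the HUD message and end-point marker direct the player to return the vehicle.
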(event `self.ReceiveBeginPlay`
  (bind _returnvalue (`|CreateWidget` "/Game/PizzaBoySystem/Widgets/W_Interaction.W_Interaction_C" null "Deliver Pizza"))
  (set `self.W_Interaction` _returnvalue)
  (`self.SetActorEnableCollision` false))

(event `Enable Delivery Point`
  (params (Enabled :type Boolean))
  (bind _staticmesh (`self.StaticMesh`))
  (if (and Enabled (`self.Can Enable?`))
    (`SceneComponent.SetHiddenInGame` _staticmesh false false)
    (`self.SetActorEnableCollision` true)
    (else
      (`SceneComponent.SetHiddenInGame` _staticmesh true false)
      (`self.SetActorEnableCollision` false))))

(event `Key|E`
  (params (Key :type "Key Structure"))
  (bind _w_message (`/Game/PizzaBoySystem/Blueprints/BP_HUD.W_Message` (`/Game/PizzaBoySystem/Blueprints/FunctionLibrary.Get HUD`)))
  (:`Pressed`
    (`/Engine/EditorBlueprintResources/StandardMacros.Gate` true :!label _label
      (:`Exit`
        (`Widget.RemoveFromParent` (`self.W_Interaction`))
        (`self.Pay Comission`)
        (`self.Deliver Pizza`)
        (`self.Enable Delivery Point` false)
        (set `self.Can Enable?` false)
        (`/Game/PizzaBoySystem/Blueprints/ActorMacroLibrary.All Delivered`
          (:`true`
            (set `/Game/PizzaBoySystem/Widgets/W_Message.Text 1` "Return the vehicle at the" _w_message)
            (set `/Game/PizzaBoySystem/Widgets/W_Message.Location Name` "Pizza Place " _w_message)
            (`/Game/PizzaBoySystem/Blueprints/BP_EndMissionTrigger.Enable Marker` (`/Game/PizzaBoySystem/Blueprints/BP_DeliveryVehicle.End Point` (`/Game/PizzaBoySystem/Blueprints/FunctionLibrary.Get Delivery Vehicle`)) true)))))))

(event `self.Sphere.OnComponentBeginOverlap`
  (params (OverlappedComponent :type "PrimitiveComponent Object Reference") (OtherActor :type "Actor Object Reference") (OtherComp :type "PrimitiveComponent Object Reference") (OtherBodyIndex :type Integer) (bFromSweep :type Boolean) (SweepResult :type "HitResult Structure (by ref)"))
  (if (== OtherActor (`/Game/PizzaBoySystem/Blueprints/FunctionLibrary.Get Delivery Vehicle`))
    (`self.EnableInput` (`GameplayStatics.GetPlayerController` 0))
    (`/Engine/EditorBlueprintResources/StandardMacros.DoOnce` false :!label _label_2
      (:`Completed`
        (`UserWidget.AddToViewport` (`self.W_Interaction`) 0)
        (goto _label :!via `Open`)))))

(event `self.Sphere.OnComponentEndOverlap`
  (params (OverlappedComponent :type "PrimitiveComponent Object Reference") (OtherActor :type "Actor Object Reference") (OtherComp :type "PrimitiveComponent Object Reference") (OtherBodyIndex :type Integer))
  (if (== (`/Game/PizzaBoySystem/Blueprints/FunctionLibrary.Get Delivery Vehicle`) OtherActor)
    (`self.DisableInput` (`GameplayStatics.GetPlayerController` 0))
    (`Widget.RemoveFromParent` (`self.W_Interaction`))
    (`|ExecutionSequence`
      (:`then_0`
        (goto _label :!via `Close`))
      (:`then_1`
        (goto _label_2 :!via `Reset`)))))

(event `Pay Comission`
  (bind _asbp_third_person_game_mode (`/Game/PizzaBoySystem/Blueprints/FunctionLibrary.Get Game Mode`))
  (set `/Game/PizzaBoySystem/Blueprints/BP_GameMode.Earnings` (+ (`/Game/PizzaBoySystem/Blueprints/BP_GameMode.Earnings` _asbp_third_person_game_mode) (`KismetMathLibrary.RandomIntegerInRange` 2 7)) _asbp_third_person_game_mode))

(event `Deliver Pizza`
  (bind _asbp_third_person_game_mode (`/Game/PizzaBoySystem/Blueprints/FunctionLibrary.Get Game Mode`))
  (set `/Game/PizzaBoySystem/Blueprints/BP_GameMode.Pizzas` (+ (`/Game/PizzaBoySystem/Blueprints/BP_GameMode.Pizzas` _asbp_third_person_game_mode) 1) _asbp_third_person_game_mode))

(fn `UserConstructionScript`)