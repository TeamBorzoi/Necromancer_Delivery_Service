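; Game mode that starts and ends timed pizza delivery missions and holds their delivery, earnings and pizza counters.
; StartMission enables the passed-in delivery targets, hides all mission trigger markers and hands the time limit to the HUD.
; EndMission removes the mission HUD and messages, shows a passed or failed widget, sends earnings to the wallet on success, then resets counters and restores markers.
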(event `Start Mission`
  (params (InputPin :type "Array of /Game/PizzaBoySystem/Blueprints/BP_DeliveryPoint Object Reference") (Minutes :type Integer) (Seconds :type Integer))
  (set `self.Pizza Mission Active?` true)
  (set `self.Deliveries` (`KismetArrayLibrary.Array_Length` InputPin))
  (`/Game/PizzaBoySystem/Blueprints/BP_HUD.Mission HUD` (`/Game/PizzaBoySystem/Blueprints/FunctionLibrary.Get HUD`) Minutes Seconds)
  (for _array_element InputPin
    (set `/Game/PizzaBoySystem/Blueprints/BP_DeliveryPoint.Can Enable?` true _array_element)
    (bind _outactors (`GameplayStatics.GetAllActorsOfClass` "/Game/PizzaBoySystem/Blueprints/BP_MissionTrigger.BP_MissionTrigger_C"))
    (for _array_element_2 _outactors
      (`/Game/PizzaBoySystem/Blueprints/BP_MissionTrigger.Enable Marker` _array_element_2 false))))

(event `End Mission`
  (params (`Mission Passed` :type Boolean))
  (bind _returnvalue (`/Game/PizzaBoySystem/Blueprints/FunctionLibrary.Get HUD`))
  (bind _earnings (`self.Earnings`))
  (set `self.Pizza Mission Active?` false)
  (`Widget.RemoveFromParent` (`/Game/PizzaBoySystem/Blueprints/BP_HUD.W_PizzaBoyHUD` _returnvalue))
  (if `Mission Passed`
    (`/Game/PizzaBoySystem/Blueprints/BP_HUD.Wallet` _returnvalue _earnings)
    (bind _returnvalue_2 (`|CreateWidget` "/Game/PizzaBoySystem/Widgets/W_MissionPassed.W_MissionPassed_C" null (`self.Deliveries`) _earnings))
    (`UserWidget.AddToViewport` _returnvalue_2 0)
    (else
      (bind _returnvalue_3 (`|CreateWidget` "/Game/PizzaBoySystem/Widgets/W_MissionFailed.W_MissionFailed_C"))
      (`UserWidget.AddToViewport` _returnvalue_3 0)))
  (set `self.Earnings` 0)
  (set `self.Deliveries` 0)
  (set `self.Pizzas` 0)
  (bind _foundwidgets (`WidgetBlueprintLibrary.GetAllWidgetsOfClass` "/Game/PizzaBoySystem/Widgets/W_Message.W_Message_C"))
  (for _array_element _foundwidgets
    (`Widget.RemoveFromParent` _array_element))
  (bind _foundwidgets_2 (`WidgetBlueprintLibrary.GetAllWidgetsOfClass` "/Game/PizzaBoySystem/Widgets/W_Message2.W_Message2_C"))
  (for _array_element_2 _foundwidgets_2
    (`Widget.RemoveFromParent` _array_element_2))
  (bind _outactors (`GameplayStatics.GetAllActorsOfClass` "/Game/PizzaBoySystem/Blueprints/BP_MissionTrigger.BP_MissionTrigger_C"))
  (for _array_element_3 _outactors
    (`/Game/PizzaBoySystem/Blueprints/BP_MissionTrigger.Enable Marker` _array_element_3 true)))

(fn `UserConstructionScript`)