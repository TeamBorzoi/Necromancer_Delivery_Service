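; BP_NecroInstance is a 2D music manager that tracks one current song through a stored audio component reference.
; PlayMusic spawns a track only when CurrentSong is not valid, so it does not interrupt an existing one.
; SwitchMusic stops any valid current song, then spawns and stores the new track, while StopMusic stops it without clearing the reference.
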(event `PlayMusic`
  (params (Music :type "SoundBase Object Reference"))
  (`self.CurrentSong`
    (:`then`)
    (:`else`
      (bind _returnvalue (`GameplayStatics.SpawnSound2D` Music 1.0 1.0 0.0 null))
      (set `self.CurrentSong` _returnvalue))))

(event `SwitchMusic`
  (params (Music :type "SoundBase Object Reference"))
  (bind _currentsong (`self.CurrentSong`)
    (:`then`
      (`AudioComponent.Stop` _currentsong))
    (:`else`
      _))
  (bind _returnvalue (`GameplayStatics.SpawnSound2D` Music 1.0 1.0 0.0 null))
  (set `self.CurrentSong` _returnvalue))

(event `StopMusic`
  (bind _currentsong (`self.CurrentSong`)
    (:`then`
      (`AudioComponent.Stop` _currentsong))
    (:`else`)))